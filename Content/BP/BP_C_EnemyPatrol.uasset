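; Patrolling enemy Blueprint that shoots the first-person player and has a health bar turned toward them by a looping timer.
; Pawn sensing snaps it toward the player and fires projectiles behind a one-second cooldown gate.
; Damage updates the widget; zero health triggers ragdoll, hides the bar and destroys the actor after a delay.
; BeginPlay picks a random patrol point, but the timeline movement logic is never triggered.
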(event OnSeePawn(PawnSensing)
  (params (Pawn :type Pawn%20Object%20Reference))
  ;[1 1 1] Shoot at Player
  (bind _asbp_first_person_character (Utilities|Casting|CastToBP_FirstPersonCharacter Pawn))
  (Utilities|FlowControl|Sequence
    (:then_0
      (Transformation|SetActorRotation (Math|Rotator|FindRelativeLookatRotation (Math|Conversions|ToTransform(Vector) (Transformation|GetActorLocation)) (Transformation|GetActorLocation _asbp_first_person_character))))
    (:then_1
      (if (Variables|Default|GetSpawnProjectile)
        (Game|SpawnActorfromClass "/Game/FirstPerson/Blueprints/BP_FirstPersonProjectile.BP_FirstPersonProjectile_C" (Transformation|GetWorldTransform (Variables|Default|GetSpawnBullet)) "Undefined" 0 0)
        (Variables|Default|SetSpawnProjectile false)
        (Utilities|FlowControl|Delay 1.0)
        (Variables|Default|SetSpawnProjectile true)))))

(event Custom|Face%20health%20bar%20towards%20player
  (bind _health_widget (Variables|Default|GetHealth%20Widget))
  ;[1 1 1] Rotate health bar towards player camera
  (Transformation|SetWorldRotation _health_widget (Math|Rotator|MakeRotator 0.0 0.0 (.yaw (Math|Rotator|FindLookatRotation (Transformation|GetWorldLocation _health_widget) (Transformation|GetActorLocation (Game|GetPlayerCharacter 0))))) false false))

(event Custom|Update%20health%20bar
  ;[1 1 1] Update health bar widget
  (bind _asui_enemy_health (Utilities|Casting|CastToUI_Enemy_Health (UserInterface|GetWidget (Variables|Default|GetHealth%20Widget))))
  (Progress|SetPercent (Variables|/Game/UI/UI_Enemy_Health.UI_Enemy_Health_C|GetPB_Health _asui_enemy_health) (/ (Variables|Default|GetCurrent%20Health) 1e+02)))

(event Custom|Death
  ;[1 1 1] Enemy death
  (Class|SkeletalMeshComponent|SetAllBodiesBelowSimulatePhysics (Variables|Character|GetMesh) (Utilities|Name|MakeLiteralName "root") true true)
  (Rendering|SetVisibility (Variables|Default|GetHealth%20Widget) false false)
  (Collision|SetCollisionResponsetoChannel (Variables|Collision|GetCapsuleComponent) "ECC_Pawn" "ECR_Ignore")
  (Utilities|FlowControl|Delay 5.0)
  (Actor|DestroyActor))

(event EventBeginPlay
  ;[1 1 1] Init
  (Utilities|FlowControl|Sequence
    (:then_0
      (Utilities|Time|SetTimerbyFunctionName 0 "Face health bar towards player" 0.1 true))
    (:then_1
      (Variables|Default|SetPatrolPoints (Utilities|Array|MakeArray (Transformation|GetWorldLocation (Variables|Default|GetMovepos1)) (Transformation|GetWorldLocation (Variables|Default|GetMovepos2)) (Transformation|GetWorldLocation (Variables|Default|GetMovepos3))))
      (CallFunction|GetRandomLoc))))

(event Game|Damage|EventAnyDamage
  (params (Damage :type Float%20%28single-precision%29) (DamageType :type Damage%20Type%20Object%20Reference) (InstigatedBy :type Controller%20Object%20Reference) (DamageCauser :type Actor%20Object%20Reference))
  ;[1 1 1] Take damage
  (Variables|Default|SetCurrent%20Health (Math|Integer|Clamp(Integer) (Math|Float|Truncate (- (Variables|Default|GetCurrent%20Health) Damage)) 0 100))
  (CallFunction|UpdateHealthBar)
  (if (<= (Variables|Default|GetCurrent%20Health) 0)
    (CallFunction|Death)))

(fn ConstructionScript)

(fn GetRandomLoc
  (Variables|Default|SetCurrentPatrolPoint (Math|Random|RandomInteger (Utilities|Array|Length (Variables|Default|GetPatrolPoints)))))